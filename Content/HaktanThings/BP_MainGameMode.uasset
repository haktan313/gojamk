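; BP_MainGameMode is a game mode that loads the Kitchen level once the player has maxed out both the Tomato and Pickle stats.
; On BeginPlay it casts the player character to BP_JoseMorinho and shows a WB_PlayerStats widget fed by that character's HStatHandler.
; It also binds to the handler's max-value event, setting a done flag per stat so the two can finish in either order.
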(event Custom|OnStatReachMaxValue_Event
  (params (statName :type String))
  (switch string statName
    (:tomato
      (bind _output_get (Variables|Default|SetbTomatoDone true))
      (if (and _output_get (Variables|Default|GetbPickleDone))
        (Game|OpenLevel(byName) "Kitchen" :!label _label)))
    (:pickle
      (bind _output_get_2 (Variables|Default|SetbPickleDone true))
      (if (and _output_get_2 (Variables|Default|GetbTomatoDone))
        (goto _label)))))

(event EventBeginPlay
  (bind _asbp_jose_morinho (Utilities|Casting|CastToBP_JoseMorinho (Game|GetPlayerCharacter 0)))
  (bind _returnvalue (UserInterface|CreateWidget "/Game/HaktanThings/WB_PlayerStats.WB_PlayerStats_C" 0 (Utilities|Map|MakeMap "Player" (Variables|/Script/gojamk.JoseMorinho|GetHStatHandler _asbp_jose_morinho))))
  (UserInterface|Viewport|AddtoViewport _returnvalue 0)
  (EventDispatchers|AssignOnStatReachMaxValue (Variables|/Script/gojamk.JoseMorinho|GetHStatHandler _asbp_jose_morinho) (delegate Custom|OnStatReachMaxValue_Event)))

(fn ConstructionScript)