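; BP_JoseMorinho is a character that triggers an ice cube ability in one of four directions.
; Pressing E traces to the floor and sends the hit actor an ice cuber message with a direction enum derived from yaw.
; An older self-contained version remains: events spawn or destroy cube rows, but their trace and timer setup is disconnected.
; Z prints the tracked cube count for debugging.
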(event Custom|IceCubes
  (bind _cubeamount (Variables|Default|GetCubeAmount))
  (bind _actorforwardvectorsave (Variables|Default|GetActorForwardVectorSave))
  (bind _returnvalue (+ _cubeamount 1))
  (bind _counter (Utilities|FlowControl|DoN _returnvalue)
    (:Exit
      (if (not (>= _counter _returnvalue))
        (Game|SpawnActorfromClass "/Game/Yunus_Folder/Blueprints/BP_IceCube.BP_IceCube_C" (Math|Transform|MakeTransform (+ (* (* (Variables|Default|GetCubeCounter) 220) _actorforwardvectorsave) (+ (Variables|Default|GetActorLocationSave) (* _actorforwardvectorsave 1.5e+02))) "0, 0, 0" "1.000000,1.000000,1.000000") "Undefined" "MultiplyWithRoot" 0 0 0)
        (Math|Integer|IncrementInt (Variables|Default|GetCubeCounter))))))

(event Custom|DestroyIceCubes
  (bind _cubes (Variables|Default|GetCubes))
  (bind _cubecounter (Variables|Default|GetCubeCounter))
  (bind _output (Utilities|Array|Get(acopy) _cubes _cubecounter))
  (Utilities|IsValid _output
    (:Is%20Valid
      (Actor|DestroyActor _output)
      (Utilities|Array|RemoveItem _cubes _output)
      (Math|Integer|IncrementInt (Variables|Default|GetCubeCounter)
        (:%20%20
          (if (Utilities|Array|IsEmpty (Variables|Default|GetCubes))
            _))))))

(event Input|KeyboardEvents|E
  (params (Key :type Key%20Structure :default "None"))
  (bind _returnvalue (Transformation|GetActorLocation))
  (bind (_x _y _z) (Class|KismetMathLibrary|BreakVector3f _returnvalue))
  (:Pressed
    (bind _outhit (Collision|LineTraceByChannel _returnvalue (Math|Vector|MakeVector _x _y (- _z 2e+02)) "TraceTypeQuery1" false 0 "ForDuration"))
    (bind _direction (CallFunction|RotationtoDirection))
    (Class|BPIIceCuber|InnitialIceCuber(Message) (.HitActor (Collision|BreakHitResult _outhit)) _direction)))

(event Input|KeyboardEvents|Z
  (params (Key :type Key%20Structure :default "None"))
  (:Pressed
    (Development|PrintString (Utilities|String|ToString(Integer) (Utilities|Array|Length (Variables|Default|GetCubes))))))

(fn ConstructionScript)

(fn RotationtoDirection
  (bind _returnvalue (Transformation|GetActorRotation))
  (bind _returnvalue_2 (Transformation|GetActorRotation))
  (bind _returnvalue_3 (Transformation|GetActorRotation))
  (if (and (>= (.yaw _returnvalue) -45.0) (<= (.yaw _returnvalue) 45.0))
    (return "NewEnumerator0")
    (elif (and (>= (.yaw _returnvalue_3) 45.0) (<= (.yaw _returnvalue_3) 135.0))
      (return "NewEnumerator3")
      (elif (and (>= (.yaw _returnvalue_2) -135.0) (<= (.yaw _returnvalue_2) -45.0))
        (return "NewEnumerator2")
        (else
          (return "NewEnumerator1"))))))