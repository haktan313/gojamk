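; BP_Grid is one cell of a five-wide grid that creates or melts lines of ice cubes in a chosen direction.
; InnitialIceCuber checks the neighboring cell, starting a spawn run if empty or a melt run if occupied.
; IceCube relays the run cell to cell through the BP_GridManager's Grids array every half second, with index checks for edges and row wrapping.
; Spawn runs stop at occupied cells, while melt runs continue past empty ones.
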(event EventBeginPlay
  (bind _returnvalue (Actor|GetActorOfClass "/Game/Yunus_Folder/Blueprints/BP_GridManager.BP_GridManager_C"))
  (Variables|Default|SetManager _returnvalue))

(event EventInnitialIceCuber
  (params (Direction :type E_Direction%20Enum :default "NewEnumerator0"))
  (bind _returnvalue (Utilities|Select :Index Direction :NewEnumerator0 -5 :NewEnumerator1 5 :NewEnumerator2 -1 :NewEnumerator3 1))
  (bind _gridindex (Variables|Default|GetGridIndex))
  (bind _manager (Variables|Default|GetManager))
  (bind _returnvalue_2 (+ _returnvalue _gridindex))
  (bind _grids (Variables|/Game/Yunus_Folder/Blueprints/BP_GridManager.BP_GridManager_C|GetGrids _manager))
  (bind _output (Utilities|Array|Get(acopy) _grids _returnvalue_2))
  (if (not (<= _returnvalue_2 -1))
    (if (== (Math|Integer|Absolute(Integer) (- _returnvalue_2 (Variables|Default|GetGridIndex))) 1)
      (if (== (/ (Variables|Default|GetGridIndex) 5) (/ _returnvalue_2 5))
        (if (not (>= _returnvalue_2 26)) :!label _label
          (if (Variables|BP_Grid_C|GetIsEmpty _output)
            (CallFunction|SpawnIceCube _output)
            (Utilities|FlowControl|Delay 0.5)
            (Default|IceCube _output Direction false)
            (else
              (CallFunction|DestroyIceCube _output)
              (Utilities|FlowControl|Delay 0.5)
              (Default|IceCube _output Direction true)))))
      (else
        (goto _label)))))

(event EventIceCube
  (params (Direction :type E_Direction%20Enum :default "NewEnumerator0") (Destroy :type Boolean))
  (bind _returnvalue (Utilities|Select :Index Direction :NewEnumerator0 -5 :NewEnumerator1 5 :NewEnumerator2 -1 :NewEnumerator3 1))
  (bind _gridindex (Variables|Default|GetGridIndex))
  (bind _manager (Variables|Default|GetManager))
  (bind _returnvalue_2 (+ _returnvalue _gridindex))
  (bind _grids (Variables|/Game/Yunus_Folder/Blueprints/BP_GridManager.BP_GridManager_C|GetGrids _manager))
  (bind _output (Utilities|Array|Get(acopy) _grids _returnvalue_2))
  (if (not (<= _returnvalue_2 -1))
    (if (not (>= _returnvalue_2 26))
      (if (== (Math|Integer|Absolute(Integer) (- _returnvalue_2 (Variables|Default|GetGridIndex))) 1)
        (if (== (/ (Variables|Default|GetGridIndex) 5) (/ _returnvalue_2 5))
          (if Destroy :!label _label
            (CallFunction|DestroyIceCube _output)
            (Utilities|FlowControl|Delay 0.5 :!label _label_2)
            (Default|IceCube _output Direction Destroy)
            (elif (Variables|BP_Grid_C|GetIsEmpty _output)
              (CallFunction|SpawnIceCube _output)
              (goto _label_2))))
        (else
          (goto _label))))))

(fn ConstructionScript)

(fn SpawnIceCube
  (bind _returnvalue (Game|SpawnActorfromClass "/Game/Yunus_Folder/Blueprints/BP_IceCube.BP_IceCube_C" (Transformation|GetWorldTransform (Variables|Default|GetScene)) "Undefined" "MultiplyWithRoot" 0 self 0))
  (Variables|Default|SetOccupyingCube _returnvalue)
  (Variables|Default|SetIsEmpty false))

(fn DestroyIceCube
  (Utilities|IsValid (Variables|Default|GetOccupyingCube)
    (:Is%20Valid
      (Default|Melt (Variables|Default|GetOccupyingCube))
      (Variables|Default|SetOccupyingCube 0)
      (Variables|Default|SetIsEmpty true))))