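; Level swapper actor that shows a widget when something overlaps its sphere and can open a configured level.
; While enabled, sphere overlap begin and end toggle the widget and the CanChangeLevel flag.
; A LevelSwap event opens the referenced level without checking that flag itself, and De-Activate clears the mesh's overlay material and disables the overlap response.
; The construction script applies the chosen static mesh.
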(event OnComponentEndOverlap(Sphere)
  (params (OverlappedComponent :type Primitive%20Component%20Object%20Reference) (OtherActor :type Actor%20Object%20Reference) (OtherComp :type Primitive%20Component%20Object%20Reference) (OtherBodyIndex :type Integer))
  (if (Variables|Default|GetEnabled)
    (Rendering|SetVisibility (Variables|Default|GetWidget) false false)
    (Variables|Default|SetCanChangeLevel false)))

(event OnComponentBeginOverlap(Sphere)
  (params (OverlappedComponent :type Primitive%20Component%20Object%20Reference) (OtherActor :type Actor%20Object%20Reference) (OtherComp :type Primitive%20Component%20Object%20Reference) (OtherBodyIndex :type Integer) (bFromSweep :type Boolean) (SweepResult :type Hit%20Result%20Structure%20%28by%20ref%29))
  (if (Variables|Default|GetEnabled)
    (Rendering|SetVisibility (Variables|Default|GetWidget) true false)
    (Variables|Default|SetCanChangeLevel true)))

(event Custom|De-Activate
  (Rendering|Material|SetOverlayMaterial (Variables|Default|GetStaticMesh) 0 :!class /Script/Engine.MeshComponent)
  (Variables|Default|SetEnabled false))

(event EventLevelSwap
  (Game|OpenLevel(byObjectReference) (Variables|Default|GetLevel)))

(fn ConstructionScript
  (Components|StaticMesh|SetStaticMesh (Variables|Default|GetStaticMesh) (Variables|Default|GetMesh)))