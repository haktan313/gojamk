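; BP_Magma is a magma piece that runs a staged, color-coded countdown before erupting.
; Blast starts a looping timer that drives a four-step DoN, shifting the cube's material from yellow through orange to red.
; The last step stops the timer, swaps material, waits briefly, then calls Errupt, which changes material again and moves it from the Manager's ongoing list to its ready list.
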(event Custom|Blast
  (bind _returnvalue (Utilities|Time|SetTimerbyEvent (delegate Custom|Timer) (Variables|Default|GetBlastTime%20/4) true)))

(event Custom|Timer
  (bind _counter (Utilities|FlowControl|DoN 4 :!label _label)
    (:Exit
      (Rendering|Material|SetMaterial (Variables|Default|GetCube) 0 (Utilities|Select :Index _counter :Option%200 "/Game/Yunus_Folder/Materials/M_Yellow.M_Yellow" :Option%201 "/Game/Yunus_Folder/Materials/M_Yellow.M_Yellow" :Option%202 "/Game/Yunus_Folder/Materials/M_Orange.M_Orange" :Option%203 "/Game/Yunus_Folder/Materials/M_Red.M_Red"))
      (if (>= _counter 4)
        (Utilities|Time|ClearandInvalidateTimerbyHandle (stale Custom|Blast _returnvalue))
        (Rendering|Material|SetMaterial (Variables|Default|GetCube) 0 "/Game/HaktanThings/lava/Material_033.Material_033")
        (Utilities|FlowControl|Delay 0.5)
        (CallFunction|Errupt)
        (goto _label Reset)))))

(fn ConstructionScript
  (Components|StaticMesh|SetStaticMesh (Variables|Default|GetCube) (Variables|Default|GetNew%20Mesh)))

(fn Errupt
  (bind _self self)
  (bind _manager (Variables|Default|GetManager))
  (Rendering|Material|SetMaterial (Variables|Default|GetCube) 0 "/Game/HaktanThings/lava/Material_024.Material_024")
  (Utilities|Array|Add (Variables|/Game/Yunus_Folder/Blueprints/BP_MagmaManager.BP_MagmaManager_C|GetReadyMagmas _manager) _self)
  (Utilities|Array|RemoveItem (Variables|/Game/Yunus_Folder/Blueprints/BP_MagmaManager.BP_MagmaManager_C|GetOngoingMagmas _manager) _self))